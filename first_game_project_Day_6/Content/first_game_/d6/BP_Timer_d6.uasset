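; Practice timer Blueprint that accumulates Tick delta seconds at normal speed and prints the raw running total every frame.
; Disconnected experiments, which never run, format that total as M:SS or MM:SS clocks intended to run at 10x speed.
; These compare nested branches in a Sequence against the FloatToStr00 helper, which floors a number and zero-pads it to two digits.
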(event `self.ReceiveTick`
  (params (DeltaSeconds :type "Float (single-precision)"))
  ;[0.15 0.15 0.15 0.5 17] delta seconds는 tick의 이벤트가 발생하는 모든 순간의  points을 나타냄. so it is practically same as real time that we see and use in reality.
  (bind _output_get (set `self.totalDeltaSeconds` (+ (`self.totalDeltaSeconds`) (* DeltaSeconds 1.0))))
  (`KismetSystemLibrary.PrintString` (`KismetStringLibrary.Conv_DoubleToString` _output_get)))

(fn `FloatToStr00`
  (params (number :type "Float (double-precision)"))
  (returns (str00 :type String))
  (bind _returnvalue (`KismetMathLibrary.FFloor` number))
  (bind _returnvalue_2 (`KismetStringLibrary.Conv_IntToString` _returnvalue))
  (if (< _returnvalue 10)
    (return (`KismetStringLibrary.Concat_StrStr` "0" _returnvalue_2))
    (else
      (return _returnvalue_2))))

(fn `UserConstructionScript`)