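; BP_LeftRight_d1_d6 is a practice actor whose Box component slides back and forth along relative X.
; While IsPlay is true, each Tick adds or subtracts a fixed step to a stored X value and applies it as the Box's relative location.
; A direction boolean flips at the upper and lower limits, so movement is per frame and not scaled by delta time.
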(event `self.Box.OnComponentBeginOverlap`
  (params (OverlappedComponent :type "PrimitiveComponent Object Reference") (OtherActor :type "Actor Object Reference") (OtherComp :type "PrimitiveComponent Object Reference") (OtherBodyIndex :type Integer) (bFromSweep :type Boolean) (SweepResult :type "HitResult Structure (by ref)"))
  ;[0.15 0.15 0.15 0.5 22] 참고
  ;; 첫 설명
)

(event `self.ReceiveTick`
  (params (DeltaSeconds :type "Float (single-precision)"))
  ;[0.15 0.15 0.15 0.5 20] 좌우로 움직이는 코드
  ;;[0.15 0.15 0.15 0.5 12] 디테일에서 기본값이 체크되어야 true 값 산출
  (if (`self.IsPlay`)
    (if (`self.오른쪽 이동 인가?`)
      ;; x의 +방향 = 오른쪽으로 이동함
      ;;;[0.15 0.15 0.15 0.5 10] x값에 100 추가 코드
      ;;;;[0.15 0.15 0.15 0.5 10] 여기서 이미 x변수는 set됨
      (set `self.X의 위치요` (+ (`self.X의 위치요`) 10.0))
      (`SceneComponent.K2_SetRelativeLocation` (`self.Box`) (`KismetMathLibrary.MakeVector` (`self.X의 위치요`)) false false)
      (if (>= (`self.X의 위치요`) 500.0)
        (set `self.오른쪽 이동 인가?` false))
      (else
        ;; x의 -방향 = 왼쪽으로 이동함
        ;;;[0.15 0.15 0.15 0.5 10] x값에 100 추가 코드
        ;;;;[0.15 0.15 0.15 0.5 10] 여기서 이미 x변수는 set됨
        (set `self.X의 위치요` (+ (`self.X의 위치요`) -10.0))
        (`SceneComponent.K2_SetRelativeLocation` (`self.Box`) (`KismetMathLibrary.MakeVector` (`self.X의 위치요`)) false false)
        (if (<= (`self.X의 위치요`) 0.0)
          (set `self.오른쪽 이동 인가?` true))))))

(event `self.ReceiveBeginPlay`
  ;[0.15 0.15 0.15 0.5 22] 참고
  ;; 플레이 화면 스트링 표시
)

(fn `UserConstructionScript`)

(fn `새 함수`)

(fn `새 함수_0`)