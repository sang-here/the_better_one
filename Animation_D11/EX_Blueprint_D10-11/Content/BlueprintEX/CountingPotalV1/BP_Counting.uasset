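; BP_Counting is a digit counter that also acts as a three-counter combination check for switching a portal.
; Its switch event advances Count, wraps it from 9 to 0 and updates a text render.
; Triggered requires Counter1–3 to all show 9 to toggle Portalgate, otherwise forces it off, then calls PotalOn.
; The dispatcher broadcasts forced-off and toggled-on states, but not toggled-off; CallCount's loop over all counters has no effect.
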(event `/Game/BlueprintEX/BPI_Switch.SwitchTriggerWithPressF`
  (set `self.count` (+ (`self.count`) 1))
  (if (== (`self.count`) 10)
    (set `self.count` 0))
  (`TextRenderComponent.K2_SetText` (`self.TextRender`) (`KismetTextLibrary.Conv_IntToText` (`self.count`))))

(event `/Game/BlueprintEX/BPI_Counting.Triggered`
  (`KismetSystemLibrary.PrintString` "pressed")
  (if (== (`/Game/BlueprintEX/CountingPotalV1/BP_Counting.count` (`self.Counter1`)) 9)
    (if (== (`/Game/BlueprintEX/CountingPotalV1/BP_Counting.count` (`self.Counter2`)) 9)
      (if (== (`/Game/BlueprintEX/CountingPotalV1/BP_Counting.count` (`self.Counter3`)) 9)
        (`KismetSystemLibrary.PrintString` "Hello")
        (`self.PortalToggle`)
        (`/Game/BlueprintEX/CountingPotalV1/BP_Portal.PotalOnOffFromCounting` (`self.PotalOn`))
        (else
          (`KismetSystemLibrary.PrintString` "no")
          (`self.PortalToggleAlwaysOff`)
          (`/Game/BlueprintEX/CountingPotalV1/BP_Portal.PotalOnOffFromCounting` (`self.PotalOn`))))
      (else
        (`KismetSystemLibrary.PrintString` "no")
        (`self.PortalToggleAlwaysOff`)
        (`/Game/BlueprintEX/CountingPotalV1/BP_Portal.PotalOnOffFromCounting` (`self.PotalOn`))))
    (else
      (`KismetSystemLibrary.PrintString` "no")
      (`self.PortalToggleAlwaysOff`)
      (`/Game/BlueprintEX/CountingPotalV1/BP_Portal.PotalOnOffFromCounting` (`self.PotalOn`)))))

(fn `CallCount`
  (`self.SwitchTriggerWithPressF`)
  (bind _outactors (`GameplayStatics.GetAllActorsOfClass` "BP_Counting_C"))
  (for _array_element _outactors
    (bind _asbp_counting (cast `/Game/BlueprintEX/CountingPotalV1/BP_Counting` _array_element))
    (if (== (`/Game/BlueprintEX/CountingPotalV1/BP_Counting.count` _asbp_counting) 9)
      _)))

(fn `PortalToggle`
  (bind _output_get (set `self.Portalgate` (not (`self.Portalgate`))))
  (if _output_get
    (`KismetSystemLibrary.PrintString` "Toggle in counting ready")
    (`self.NewEventDispatcherFromCounting` _output_get)))

(fn `PortalToggleAlwaysOff`
  (bind _output_get (set `self.Portalgate` false))
  (`self.NewEventDispatcherFromCounting` _output_get))

(fn `UserConstructionScript`)