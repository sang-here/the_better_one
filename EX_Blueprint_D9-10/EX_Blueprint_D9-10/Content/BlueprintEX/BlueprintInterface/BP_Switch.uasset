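; BP_Switch is an interactive lever switch that flips a Toggle boolean when triggered by an F press and broadcasts the new state through an event dispatcher.
; A self-restarting Timeline, started by the Completed event, continually steps the pivot's pitch toward positive or negative 45 degrees according to Toggle.
; The Timeline serves as a looping tick, adding fixed rotation increments until the limit is reached.
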(event `/Game/BlueprintEX/BPI_Switch.SwitchTriggerWithPressF`
  (`KismetSystemLibrary.PrintString` "pressed in switch")
  (`self.SetToggleAndSendTheDataViaDispatcher`))

(event `/Game/BlueprintEX/BPI_Portal.completed`
  (bind _returnvalue (* 1.0 10.0))
  (`Timeline|Timeline` :!label _label
    (:`Update`
      (if (`self.Toggle`)
        (if (not (>= (.pitch (.rotation (`SceneComponent.GetRelativeTransform` (`self.SwitchRotationPivot`)))) 45.0))
          (`SceneComponent.K2_AddRelativeRotation` (`self.SwitchRotationPivot`) (`KismetMathLibrary.MakeRotator` 0.0 (* _returnvalue 1.0)) false false))
        (elif (not (<= (.pitch (.rotation (`SceneComponent.GetRelativeTransform` (`self.SwitchRotationPivot`)))) -45.0))
          (`SceneComponent.K2_AddRelativeRotation` (`self.SwitchRotationPivot`) (`KismetMathLibrary.MakeRotator` 0.0 (* _returnvalue -1.0)) false false))))
    (:`Finished`
      (goto _label :!via `PlayFromStart`))))

(fn `SetToggleAndSendTheDataViaDispatcher`
  (bind _output_get (set `self.Toggle` (not (`self.Toggle`))))
  (`self.NewEventDispatcher_Toggle` _output_get))

(fn `UserConstructionScript`)