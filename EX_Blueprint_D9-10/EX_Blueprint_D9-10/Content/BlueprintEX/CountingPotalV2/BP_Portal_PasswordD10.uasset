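; Password portal that shows its Sphere when every CountingBox counter matches the Password entry at the same index.
; BeginPlay hides the Sphere, and OnPotal sets its visibility from 369ByArray, which returns false on the first mismatch.
; An older V1 event driven by PortalOnOff remains.
; FromCountingToggle's dispatcher-binding loop is disconnected, so nothing in this graph binds or calls OnPotal.
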(event `CustomEvent`
  (bind _portalonoff (`self.PortalOnOff`))
  ; V1
  (`KismetSystemLibrary.PrintString` "@@@@@@")
  (if _portalonoff
    (`SceneComponent.SetVisibility` (`self.Sphere`) _portalonoff false)
    (else
      (`SceneComponent.SetVisibility` (`self.Sphere`) _portalonoff false))))

(event `OnPotal`
  ; V2
  (bind _newparam (`self.369 by array`))
  (`KismetSystemLibrary.PrintString` "@@@@@@")
  (`SceneComponent.SetVisibility` (`self.Sphere`) _newparam false))

(event `self.ReceiveBeginPlay`
  ; V2
  (`SceneComponent.SetVisibility` (`self.Sphere`) false false)
  (`self.FromCountingToggle`))

(fn `369 by array`
  (returns (NewParam :type Boolean))
  (for (_array_element _array_index) (`self.CountingBox`)
    (if (not (== (`/Game/BlueprintEX/CountingPotalV2/BP_Counting_PasswordD10.count` _array_element) (`|GetArrayItem` (`self.password`) _array_index)))
      (return false)))
  (return true))

(fn `BP_Portal_d10_AutoGenFunc`
  (params (PortalOnOff :type Boolean))
  (set `self.PortalOnOff` PortalOnOff))

(fn `FromCountingToggle`)

(fn `UserConstructionScript`)