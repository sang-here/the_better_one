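; BP_PlayerState holds the player's health and coin count for a coin game exercise.
; HP starts at max; damage and heal functions skip when dead, apply limits and broadcast updates through a dispatcher, while FullHeal restores max directly.
; AddCoin increments and broadcasts P1Coin; GetAllCoin and the identical SubtractCount count BP_Coin actors.
; HealTillHundred currently adds zero, ignoring its Heal input, and unused alternative versions remain unwired.
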(event `self.ReceiveBeginPlay`
  (set `self.CurrentHP` (`self.MaxHp`)))

(fn `AddCoin`
  (locals (AddCoinn :type Integer) (NewLocalVar :type "Character Object Reference"))
  (bind _output_get (set `self.P1Coin` (+ (`self.P1Coin`) 1)))
  (`self.PlayerStateNewEventDispatcher_CoinAdd` _output_get))

(fn `AddDamageWithLimitZero`
  (params (Damage :type "Float (double-precision)"))
  ; V1
  (if (not (`self.IsDead`))
    (set `self.CurrentHP` (- (`self.CurrentHP`) Damage))
    (`self.DamageLimit`)
    (`self.NewEventDispatcher_UpdateHp` (`self.CurrentHP`) (`self.MaxHp`))))

(fn `DamageLimit`
  (bind _currenthp (`self.CurrentHP`))
  (if (<= _currenthp 0.0)
    (bind _output_get (set `self.CurrentHP` 0.0))
    (`KismetSystemLibrary.PrintString` (`KismetStringLibrary.Concat_StrStr` "HP: " (`KismetStringLibrary.Conv_DoubleToString` _output_get)))
    (return)
    (else
      (`KismetSystemLibrary.PrintString` (`KismetStringLibrary.Concat_StrStr` "HP: " (`KismetStringLibrary.Conv_DoubleToString` _currenthp)))
      (return))))

(fn `FullHeal`
  (set `self.CurrentHP` (`self.MaxHp`))
  (`self.NewEventDispatcher_UpdateHp` (`self.CurrentHP`) (`self.MaxHp`)))

(fn `GetAllCoin`
  (returns (TotalCoin :type Integer))
  (locals (coin :type Integer))
  (bind _outactors (`GameplayStatics.GetAllActorsOfClass` "/Game/CoinGameExercise/BP_Coin.BP_Coin_C"))
  (for _ _outactors
    (set `local.coin` (+ (`local.coin`) 1)))
  (return (`local.coin`)))

(fn `HealLimit`
  (bind _currenthp (`self.CurrentHP`))
  (if (>= _currenthp 100.0)
    (bind _output_get (set `self.CurrentHP` (`self.MaxHp`)))
    (`KismetSystemLibrary.PrintString` (`KismetStringLibrary.Concat_StrStr` "HP: " (`KismetStringLibrary.Conv_DoubleToString` _output_get)))
    (else
      (`KismetSystemLibrary.PrintString` (`KismetStringLibrary.Concat_StrStr` "HP: " (`KismetStringLibrary.Conv_DoubleToString` _currenthp))))))

(fn `HealTillHundred`
  (params (Heal :type "Float (double-precision)"))
  ; V1
  (if (not (`self.IsDead`))
    (set `self.CurrentHP` (+ (`self.CurrentHP`) 0.0))
    (`self.HealLimit`)
    (`self.NewEventDispatcher_UpdateHp` (`self.CurrentHP`) (`self.MaxHp`))))

(fn `IsDead`
  (returns (IsDeath :type Boolean))
  (return (<= (`self.CurrentHP`) 0.0)))

(fn `SubtractCount`
  (returns (TotalCoin :type Integer))
  (locals (Coin :type Integer))
  (bind _outactors (`GameplayStatics.GetAllActorsOfClass` "/Game/CoinGameExercise/BP_Coin.BP_Coin_C"))
  (for _ _outactors
    (set `local.Coin` (+ (`local.Coin`) 1)))
  (return (`local.Coin`)))

(fn `UserConstructionScript`)