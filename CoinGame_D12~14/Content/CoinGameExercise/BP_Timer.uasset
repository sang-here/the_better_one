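; BP_Timer is an actor in the coin game exercise that displays elapsed time on a text render component.
; Tick accumulates delta seconds, builds a colon-separated string from total divided by 60 and total modulo 1.0, and prints the raw total for debugging.
; FloatToStrZeroN floors and zero-pads each part, so the field after the colon always reads "00" rather than counting seconds.
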(event `self.ReceiveTick`
  (params (DeltaSeconds :type "Float (single-precision)"))
  (bind _output_get (set `self.TotalDeltalSeconds` (+ DeltaSeconds (`self.TotalDeltalSeconds`))))
  (`TextRenderComponent.K2_SetText` (`self.TextRender`) (`KismetTextLibrary.Conv_StringToText` (`KismetStringLibrary.Concat_StrStr` (`self.FloatToStrZeroN` (/ _output_get 60.0)) ":" (`self.FloatToStrZeroN` (mod _output_get 1.0)))))
  (`KismetSystemLibrary.PrintString` (`KismetStringLibrary.Conv_DoubleToString` (`self.TotalDeltalSeconds`))))

(fn `FloatToStrZeroN`
  (params (A :type "Float (double-precision)"))
  (returns (ReturnValue :type String))
  (bind _returnvalue (`KismetMathLibrary.FFloor` A))
  (bind _returnvalue_2 (`KismetStringLibrary.Conv_IntToString` _returnvalue))
  (if (< _returnvalue 10)
    (return (`KismetStringLibrary.Concat_StrStr` "0" _returnvalue_2))
    (else
      (return _returnvalue_2))))

(fn `UserConstructionScript`)