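; Switch actor that starts and stops the movers referenced in its Actors array, labelled with its display name.
; Overlap-signature handlers drive targets through either per-class cast chains or the BPI_PlayStop interface; the cast logic also exists as separate, uncalled functions.
; PressF flips Toggle and broadcasts it through the ToggleSwitch dispatcher, while another custom event flips it and calls the interface start/stop functions directly.
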(event `CustomEvent`
  (params (OverlappedComponent :type "PrimitiveComponent Object Reference") (OtherActor :type "Actor Object Reference") (OtherComp :type "PrimitiveComponent Object Reference") (OtherBodyIndex :type Integer) (bFromSweep :type Boolean) (SweepResult :type "HitResult Structure (by ref)"))
  ; 4.액터 레퍼런스와 각 액터를 판단 하는 cast를 이용하여 스위치에 connect
  (for _array_element (`self.actors`)
    ;;[0.15 0.15 0.15 0.5 12] cast 너 뉘기야
    (bind _asbp_left_right_d_1_d_6 (cast `/Game/first_game_/d6/BP_LeftRight_d1_d6` _array_element)
      (:`then`
        (set `/Game/first_game_/d6/BP_LeftRight_d1_d6.IsPlay` true _asbp_left_right_d_1_d_6))
      (:`CastFailed`
        (bind _asbp_left_right_timeline_d_6 (cast `/Game/first_game_/d6/BP_left_right_timeline_d6` _array_element)
          (:`then`
            (`/Game/first_game_/d6/BP_left_right_timeline_d6.DoPlay` _asbp_left_right_timeline_d_6))
          (:`CastFailed`
            (bind _asbp_move_ract_2_d_3_d_6 (cast `/Game/first_game_/d6/BP_moveRact2_d3_d6` _array_element)
              (:`then`
                (set `/Game/first_game_/d6/BP_moveRact2_d3_d6.lever` true _asbp_move_ract_2_d_3_d_6))
              (:`CastFailed`
                (bind _asbp_move_left_timeline__d_4_d_6 (cast `/Game/first_game_/d6/BP_move_left_Timeline__d4_d6` _array_element))
                (`/Game/first_game_/d6/BP_move_left_Timeline__d4_d6.we do it` _asbp_move_left_timeline__d_4_d_6)))))))))

(event `CustomEvent_1`
  (params (OverlappedComponent :type "PrimitiveComponent Object Reference") (OtherActor :type "Actor Object Reference") (OtherComp :type "PrimitiveComponent Object Reference") (OtherBodyIndex :type Integer))
  ; 4.액터 레퍼런스와 각 액터를 판단 하는 cast를 이용하여 스위치에 connect
  (for _array_element (`self.actors`)
    (bind _asbp_left_right_d_1_d_6 (cast `/Game/first_game_/d6/BP_LeftRight_d1_d6` _array_element)
      (:`then`
        (set `/Game/first_game_/d6/BP_LeftRight_d1_d6.IsPlay` false _asbp_left_right_d_1_d_6))
      (:`CastFailed`
        (bind _asbp_left_right_timeline_d_6 (cast `/Game/first_game_/d6/BP_left_right_timeline_d6` _array_element)
          (:`then`
            (`/Game/first_game_/d6/BP_left_right_timeline_d6.DoStop` _asbp_left_right_timeline_d_6))
          (:`CastFailed`
            (bind _asbp_move_ract_2_d_3_d_6 (cast `/Game/first_game_/d6/BP_moveRact2_d3_d6` _array_element)
              (:`then`
                (set `/Game/first_game_/d6/BP_moveRact2_d3_d6.lever` false _asbp_move_ract_2_d_3_d_6))
              (:`CastFailed`
                (bind _asbp_move_left_timeline__d_4_d_6 (cast `/Game/first_game_/d6/BP_move_left_Timeline__d4_d6` _array_element))
                (`/Game/first_game_/d6/BP_move_left_Timeline__d4_d6.we don't do it` _asbp_move_left_timeline__d_4_d_6)))))))))

(event `CustomEvent_2`
  (params (OverlappedComponent :type "PrimitiveComponent Object Reference") (OtherActor :type "Actor Object Reference") (OtherComp :type "PrimitiveComponent Object Reference") (OtherBodyIndex :type Integer) (bFromSweep :type Boolean) (SweepResult :type "HitResult Structure (by ref)"))
  ; 4.액터 레퍼런스와 각 액터를 판단 하는 cast를 이용하여 스위치에 connect / collapse to function
  (`self.interface_모든 연결된 액터들 움직이기 시작_0`))

(event `CustomEvent_4`
  ; PressF를 이용해서 오배랩 후 조종
  (bind _output_get (set `self.Toggle` (not (`self.Toggle`))))
  (if _output_get
    (`self.interface_모든 연결된 액터들 움직이기 시작_0`)
    (else
      (`self.interface_모든 연결된 액터들 움직이기 멈춤_0`))))

(event `CustomEvent_3`
  (params (OverlappedComponent :type "PrimitiveComponent Object Reference") (OtherActor :type "Actor Object Reference") (OtherComp :type "PrimitiveComponent Object Reference") (OtherBodyIndex :type Integer))
  ; 4.액터 레퍼런스와 각 액터를 판단 하는 cast를 이용하여 스위치에 connect / collapse to function
  (`self.interface_모든 연결된 액터들 움직이기 멈춤_0`))

(event `/Game/first_game_/d8_PressF/BPI_Switch.PressF`
  ; D9 // PressF를 이용해서 오배랩 후 조종
  (bind _output_get (set `self.Toggle` (not (`self.Toggle`))))
  (`self.NewEventDispatcher_ToggleSwitch` _output_get))

(fn `DoPlayAndStop0`
  (params (DoPlay :type Boolean))
  (returns (Return :type Boolean))
  (return false))

(fn `interface_모든 연결된 액터들 움직이기 멈춤_0`
  (for _array_element (`self.actors`)
    (bind _asbp_play_stop (cast `/Game/first_game_/d7/BPI_PlayStop` _array_element))
    (`/Game/first_game_/d7/BPI_PlayStop.DoPlayAndStop0` _asbp_play_stop false)))

(fn `interface_모든 연결된 액터들 움직이기 시작_0`
  (for _array_element (`self.actors`)
    (bind _asbp_play_stop (cast `/Game/first_game_/d7/BPI_PlayStop` _array_element))
    ;[0.15 0.15 0.15 0.5 12] 월드에서도 연결되는 액터들을 스위치 속의 각각 변수로도 지정을  해주어야 함
    (`/Game/first_game_/d7/BPI_PlayStop.DoPlayAndStop0` _asbp_play_stop true)))

(fn `UserConstructionScript`
  (`TextRenderComponent.K2_SetText` (`self.TextRender`) (`KismetTextLibrary.Conv_StringToText` (`KismetSystemLibrary.GetDisplayName` self))))

(fn `모든 연결된 액터들 움직이기 멈춤`
  (for _array_element (`self.actors`)
    (bind _asbp_left_right_d_1_d_6 (cast `/Game/first_game_/d6/BP_LeftRight_d1_d6` _array_element)
      (:`then`
        (set `/Game/first_game_/d6/BP_LeftRight_d1_d6.IsPlay` false _asbp_left_right_d_1_d_6))
      (:`CastFailed`
        (bind _asbp_left_right_timeline_d_6 (cast `/Game/first_game_/d6/BP_left_right_timeline_d6` _array_element)
          (:`then`
            (`/Game/first_game_/d6/BP_left_right_timeline_d6.DoStop` _asbp_left_right_timeline_d_6))
          (:`CastFailed`
            (bind _asbp_move_ract_2_d_3_d_6 (cast `/Game/first_game_/d6/BP_moveRact2_d3_d6` _array_element)
              (:`then`
                (set `/Game/first_game_/d6/BP_moveRact2_d3_d6.lever` false _asbp_move_ract_2_d_3_d_6))
              (:`CastFailed`
                (bind _asbp_move_left_timeline__d_4_d_6 (cast `/Game/first_game_/d6/BP_move_left_Timeline__d4_d6` _array_element))
                (`/Game/first_game_/d6/BP_move_left_Timeline__d4_d6.we don't do it` _asbp_move_left_timeline__d_4_d_6)))))))))

(fn `모든 연결된 액터들 움직이기 시작`
  (for _array_element (`self.actors`)
    ;[0.15 0.15 0.15 0.5 12] cast 너 뉘기야
    (bind _asbp_left_right_d_1_d_6 (cast `/Game/first_game_/d6/BP_LeftRight_d1_d6` _array_element)
      (:`then`
        (set `/Game/first_game_/d6/BP_LeftRight_d1_d6.IsPlay` true _asbp_left_right_d_1_d_6))
      (:`CastFailed`
        (bind _asbp_left_right_timeline_d_6 (cast `/Game/first_game_/d6/BP_left_right_timeline_d6` _array_element)
          (:`then`
            (`/Game/first_game_/d6/BP_left_right_timeline_d6.DoPlay` _asbp_left_right_timeline_d_6))
          (:`CastFailed`
            (bind _asbp_move_ract_2_d_3_d_6 (cast `/Game/first_game_/d6/BP_moveRact2_d3_d6` _array_element)
              (:`then`
                (set `/Game/first_game_/d6/BP_moveRact2_d3_d6.lever` true _asbp_move_ract_2_d_3_d_6))
              (:`CastFailed`
                (bind _asbp_move_left_timeline__d_4_d_6 (cast `/Game/first_game_/d6/BP_move_left_Timeline__d4_d6` _array_element))
                (`/Game/first_game_/d6/BP_move_left_Timeline__d4_d6.we do it` _asbp_move_left_timeline__d_4_d_6)))))))))