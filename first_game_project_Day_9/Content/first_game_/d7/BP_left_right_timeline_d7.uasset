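; Actor that ping-pongs its Cube between relative positions using a timeline scaled along X and Z, controlled by play/stop calls or a switch.
; Each time the timeline finishes, IsRight flips and playback alternates between Play and Reverse.
; DoPlayAndStop0 routes a boolean to DoPlay or DoStop.
; BeginPlay binds to the Switch's event dispatcher, and EventSwitchToggle repeats the same play/stop logic.
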(event `DoPlay`
  ; 와리가리 새로운 코드 D5
  ;;[0.15 0.15 0.15 0.5 10] 개발자 의도가 담기는 커스텀 이벤트 D6
  (if (`self.is_right`) :!label _label
    (bind (_direction _value) (`Timeline|타임라인` :!label _label_2)
      (:`Update`
        (`SceneComponent.K2_SetRelativeLocation` (`self.cube`) (* _value (100.0 0.0 100.0)) false false))
      (:`Finished`
        (set `self.is_right` (not (`self.is_right`)))
        (goto _label)))
    (else
      (goto _label_2 :!via `Reverse`))))

(event `DoStop`
  ; 와리가리 새로운 코드 D5
  (goto _label_2 :!via `Stop`))

(event `EventSwitchToggle`
  (params (Toggle :type Boolean))
  (if Toggle
    ; 와리가리 새로운 코드 D9 Event Dispatcher
    (if (`self.is_right`) :!label _label_3
      (bind (_direction _value) (`Timeline|Timeline` :!label _label_4)
        (:`Update`
          (`SceneComponent.K2_SetRelativeLocation` (`self.cube`) (* _value (100.0 0.0 100.0)) false false))
        (:`Finished`
          (set `self.is_right` (not (`self.is_right`)))
          (goto _label_3)))
      (else
        (goto _label_4 :!via `Reverse`)))
    (else
      (goto _label_4 :!via `Stop`))))

(event `self.ReceiveBeginPlay`
  (add `/Game/first_game_/d7/BP_switch_d7.NewEventDispatcher_ToggleSwitch` (`self.Switch`) (`|CreateDelegate` :!event `EventSwitchToggle`)))

(fn `DoPlayAndStop0`
  (params (DoPlay :type Boolean))
  (returns (Return :type Boolean))
  (if DoPlay
    (`self.DoPlay`)
    (else
      (`self.DoStop`)))
  (return false))

(fn `UserConstructionScript`)