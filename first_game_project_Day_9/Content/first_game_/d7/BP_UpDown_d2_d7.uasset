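; BP_UpDown_d2_d7 is an event dispatcher exercise actor whose Cone bobs up and down when switched on.
; On BeginPlay it binds to the referenced Switch's toggle dispatcher, with EventSwitchToggle setting the IsPlay flag.
; While playing, Tick steps the cone's relative Z by a fixed, frame-rate-dependent amount, reversing at height limits.
; DoPlayAndStop0 also sets IsPlay directly.
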(event `self.ReceiveTick`
  (params (DeltaSeconds :type "Float (single-precision)"))
  ; D9 EventDispatcher 위아래로 움직이는 코드
  ;;[0.15 0.15 0.15 0.5 12] switch로 호출
  (if (`self.IsPlay`)
    (if (`self.Is_Move_up`)
      (set `self.Loc_Z` (+ (`self.Loc_Z`) 5.0))
      (`SceneComponent.K2_SetRelativeLocation` (`self.Cone`) (`KismetMathLibrary.MakeVector` 0.0 0.0 (`self.Loc_Z`)) false false)
      (if (>= (`self.Loc_Z`) 250.0)
        (set `self.Is_Move_up` false))
      (else
        (set `self.Loc_Z` (+ (`self.Loc_Z`) -5.0))
        (`SceneComponent.K2_SetRelativeLocation` (`self.Cone`) (`KismetMathLibrary.MakeVector` 0.0 0.0 (`self.Loc_Z`)) false false)
        (if (<= (`self.Loc_Z`) 0.0)
          (set `self.Is_Move_up` true))))))

(event `self.ReceiveBeginPlay`
  (add `/Game/first_game_/d7/BP_switch_d7.NewEventDispatcher_ToggleSwitch` (`self.Switch`) (`|CreateDelegate` :!event `EventSwitchToggle`)))

(fn `DoPlayAndStop0`
  (params (DoPlay :type Boolean))
  (returns (Return :type Boolean))
  (set `self.IsPlay` DoPlay)
  (return false))

(fn `EventSwitchToggle`
  (params (Toggle :type Boolean))
  (set `self.IsPlay` Toggle))

(fn `UserConstructionScript`)