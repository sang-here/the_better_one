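; Player state for a coin game that tracks the player's collected coins and counts the coin actors in the level.
; AddCoin increments P1Coin and broadcasts the new total through an event dispatcher.
; GetAllCoin and SubtractCount share identical logic, looping over all BP_Coin actors to increment and return Coin; despite its name, SubtractCount subtracts nothing.
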(event `self.ReceiveBeginPlay`)

(fn `AddCoin`
  (locals (AddCoinn :type Integer) (NewLocalVar :type "Character Object Reference"))
  (bind _output_get (set `self.P1Coin` (+ (`self.P1Coin`) 1)))
  (`self.PlayerStateNewEventDispatcher` _output_get))

(fn `GetAllCoin`
  (returns (TotalCoin :type Integer))
  (locals (coin :type Integer))
  (bind _outactors (`GameplayStatics.GetAllActorsOfClass` "/Game/CoinGameExercise/BP_Coin.BP_Coin_C"))
  (for _ _outactors
    (set `local.coin` (+ (`local.coin`) 1)))
  (return (`local.coin`)))

(fn `SubtractCount`
  (returns (TotalCoin :type Integer))
  (locals (Coin :type Integer))
  (bind _outactors (`GameplayStatics.GetAllActorsOfClass` "/Game/CoinGameExercise/BP_Coin.BP_Coin_C"))
  (for _ _outactors
    (set `local.Coin` (+ (`local.Coin`) 1)))
  (return (`local.Coin`)))

(fn `UserConstructionScript`)