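; BP_LeftRight is an event dispatcher example that slides a Cube back and forth along local X while toggled on.
; On BeginPlay it binds to a referenced Switch's toggle dispatcher, with SwitchToggle as the apparent handler setting Toggle.
; While Toggle is set, Tick moves the cube by a fixed, frame-rate-dependent step, flipping LeftOrRight at each end of its range.
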(event `self.ReceiveTick`
  (params (DeltaSeconds :type "Float (single-precision)"))
  (if (`self.Toggle`)
    (if (`self.LeftOrRight`)
      (`self.LeftXdelta-10Till-350`)
      (else
        (`self.RightXdelta10Till0`)))))

(event `self.ReceiveBeginPlay`
  (`self.GetDataFromDispatcherOfSwitch`))

(fn `GetDataFromDispatcherOfSwitch`
  (add `/Game/BlueprintEX/BlueprintInterface/BP_Switch.NewEventDispatcher_Toggle` (`self.Switch`) (`|CreateDelegate` :!event `SwitchToggle`)))

(fn `LeftXdelta-10Till-350`
  (set `self.X` (+ (`self.X`) -10.0))
  (`SceneComponent.K2_SetRelativeLocation` (`self.Cube`) (`KismetMathLibrary.MakeVector` (`self.X`)) false false)
  (if (< (`self.X`) -350.0)
    (set `self.LeftOrRight` false)))

(fn `RightXdelta10Till0`
  (set `self.X` (+ (`self.X`) 10.0))
  (`SceneComponent.K2_SetRelativeLocation` (`self.Cube`) (`KismetMathLibrary.MakeVector` (`self.X`)) false false)
  (if (> (`self.X`) 0.0)
    (set `self.LeftOrRight` true)))

(fn `SwitchToggle`
  (params (NewParam :type Boolean))
  (set `self.Toggle` NewParam))

(fn `UserConstructionScript`)