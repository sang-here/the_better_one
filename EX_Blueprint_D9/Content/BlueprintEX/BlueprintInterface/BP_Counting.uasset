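; BP_Counting is a counter puzzle actor whose correct combination signals a portal gate.
; Each SwitchTriggerwithPressF increments Count and updates its text, except when wrapping past nine to zero, which leaves the text unchanged.
; Completed checks three referenced counters for nines, then calls PortalToggle, which flips Portalgate and fires an event dispatcher only when true.
; CallCount also scans all BP_Counting actors, but its check does nothing.
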(event `/Game/BlueprintEX/BPI_Switch.SwitchTriggerWithPressF`
  (set `self.count` (+ (`self.count`) 1))
  (if (> (`self.count`) 9)
    (set `self.count` 0)
    (else
      (`TextRenderComponent.K2_SetText` (`self.TextRender`) (`KismetTextLibrary.Conv_IntToText` (`self.count`))))))

(event `/Game/BlueprintEX/BPI_Portal.Completed`
  (`KismetSystemLibrary.PrintString` "pressed")
  (if (== (`/Game/BlueprintEX/BlueprintInterface/BP_Counting.count` (`self.Counter1`)) 9)
    (if (== (`/Game/BlueprintEX/BlueprintInterface/BP_Counting.count` (`self.Counter2`)) 9)
      (if (== (`/Game/BlueprintEX/BlueprintInterface/BP_Counting.count` (`self.Counter3`)) 9)
        (`KismetSystemLibrary.PrintString` "Hello")
        (`self.PortalToggle`)
        (else
          (`KismetSystemLibrary.PrintString` "no")))
      (else
        (`KismetSystemLibrary.PrintString` "no")))
    (else
      (`KismetSystemLibrary.PrintString` "no"))))

(fn `CallCount`
  (`self.SwitchTriggerWithPressF`)
  (bind _outactors (`GameplayStatics.GetAllActorsOfClass` "BP_Counting_C"))
  (for _array_element _outactors
    (bind _asbp_counting (cast `/Game/BlueprintEX/BlueprintInterface/BP_Counting` _array_element))
    (if (== (`/Game/BlueprintEX/BlueprintInterface/BP_Counting.count` _asbp_counting) 9)
      _)))

(fn `PortalToggle`
  (bind _output_get (set `self.Portalgate` (not (`self.Portalgate`))))
  (if _output_get
    (`KismetSystemLibrary.PrintString` "Toggle in counting ready")
    (`self.NewEventDispatcherFromCounting` _output_get)))

(fn `UserConstructionScript`)