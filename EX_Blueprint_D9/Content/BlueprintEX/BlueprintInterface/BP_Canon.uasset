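; BP_Canon is a switchable cannon that repeatedly fires BP_CanonBall actors from its Arrow component.
; The SwitchTriggerwithPressF event flips a toggle, either firing at once and starting a looping one-second timer, or clearing that timer.
; The timer calls CanonShooter by function name to spawn each ball at the Arrow's world location and rotation.
; Other timer nodes sit unconnected in the event graph.
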(event `/Game/BlueprintEX/BPI_Switch.SwitchTriggerWithPressF`
  (bind _output_get (set `self.Toggle` (not (`self.Toggle`))))
  (if _output_get
    (`KismetSystemLibrary.K2_SetTimer` null "CanonShooter" 1.0 true)
    (`self.CanonShooter`)
    (else
      (`KismetSystemLibrary.K2_ClearTimer` null "CanonShooter"))))

(fn `CanonShooter`
  (bind (_returnvalue_location _returnvalue_rotation) (`KismetMathLibrary.BreakTransform` (`SceneComponent.K2_GetComponentToWorld` (`self.Arrow`))))
  (`|SpawnActorFromClass` "/Game/BlueprintEX/BlueprintInterface/BP_CanonBall.BP_CanonBall_C" (`KismetMathLibrary.MakeTransform` _returnvalue_location _returnvalue_rotation) "Undefined" "MultiplyWithRoot" null null))

(fn `UserConstructionScript`)