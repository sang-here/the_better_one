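; Practice actor that moves a Cube back and forth along a timeline-driven path, switched on and off by a linked Switch.
; BeginPlay binds to the Switch's toggle dispatcher, and a custom Toggle event plays or stops the timeline.
; Each update sets the cube's relative location from the scaled timeline vector, and finishing restarts it to loop.
; The Toggle and DoPlayAndStop0 functions are empty stubs.
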(event `CustomEvent`
  (params (Toggle :type Boolean))
  ; 와리가리 새로운 코드 D5
  ;;[0.15 0.15 0.15 0.5 12] D6
  (if Toggle
    (bind (_direction _vector) (`Timeline|타임라인` :!label _label)
      (:`Update`
        (`SceneComponent.K2_SetRelativeLocation` (`self.cube`) (* _vector 500.0) false false))
      (:`Finished`
        (goto _label :!via `PlayFromStart`)))
    (else
      (goto _label :!via `Stop`))))

(event `self.ReceiveBeginPlay`
  (add `/Game/first_game_/d7/BP_switch_d7.NewEventDispatcher_ToggleSwitch` (`self.Switch`) (`|CreateDelegate` :!event `CustomEvent`)))

(fn `DoPlayAndStop0`
  (params (DoPlay :type Boolean))
  (returns (Return :type Boolean))
  (if DoPlay
    _))

(fn `Toggle`
  (params (Toggle :type Boolean)))

(fn `UserConstructionScript`)