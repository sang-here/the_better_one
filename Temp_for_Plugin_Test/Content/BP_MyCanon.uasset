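; Cannon Blueprint that spins its Barrels component and repeatedly fires BP_BlackBall actors from an ejection arrow.
; BeginPlay flips Toggle to either start, or clear the timers and stop the looping spin.
; Timeline_1 ramps rotation with a sine ease and re-sets both looping shooter timers every update, then Timeline_2 sustains the spin.
; Fastforward scales spin and fire rate; the CanonBallShellShooter timer target is not defined here.
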(event `self.ReceiveBeginPlay`
  (bind _output_get (set `self.Toggle` (not (`self.Toggle`))))
  (if _output_get
    (bind (_direction _sine) (`Timeline|Timeline_1`)
      (:`Update`
        (`SceneComponent.K2_AddRelativeRotation` (`self.Barrels`) (`KismetMathLibrary.MakeRotator` 0.0 0.0 (* (* (`KismetMathLibrary.DegSin` (* _sine (/ (`KismetMathLibrary.GetPI`) 2.0))) -10.0) (* 1.0 (`self.Fastforward`)))) false false)
        (`KismetSystemLibrary.K2_SetTimer` null "CanonBallShellShooter" (/ 1.0 (`self.Fastforward`)) true)
        (`KismetSystemLibrary.K2_SetTimer` null "CanonShooter" (/ 1.0 (`self.Fastforward`)) true))
      (:`Finished`
        (bind (_direction_2 _sine_2) (`Timeline|Timeline_2` :!label _label)
          (:`Update`
            (`SceneComponent.K2_AddRelativeRotation` (`self.Barrels`) (`KismetMathLibrary.MakeRotator` 0.0 0.0 (* (* _sine_2 -10.0) (* 1.0 (`self.Fastforward`)))) false false))
          (:`Finished`
            (goto _label :!via `PlayFromStart`)))))
    (else
      (`|ExecutionSequence`
        (:`then_0`
          (`KismetSystemLibrary.K2_ClearTimer` null "CanonBallShellShooter")
          (`KismetSystemLibrary.K2_ClearTimer` null "CanonShooter"))
        (:`then_1`
          (goto _label :!via `Stop`))))))

(fn `CanonShooter`
  (bind (_returnvalue_location _returnvalue_rotation) (`KismetMathLibrary.BreakTransform` (`SceneComponent.K2_GetComponentToWorld` (`self.CanonBallEjectionPointArrow`))))
  (`|SpawnActorFromClass` "/Game/BP_BlackBall.BP_BlackBall_C" (`KismetMathLibrary.MakeTransform` _returnvalue_location _returnvalue_rotation) "Undefined" "MultiplyWithRoot" null null))

(fn `UserConstructionScript`
  (`parent.UserConstructionScript`))