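; Example actor for event dispatchers that moves its Cube around a square path in the XZ plane while Toggle is on.
; BeginPlay binds to the Switch's toggle dispatcher, presumably to SwitchToggle, which sets Toggle.
; Tick uses MoveType as a four-state machine, each state stepping the cube and advancing past its X or Z limit.
; Steps are fixed per frame, so speed depends on frame rate.
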(event `self.ReceiveTick`
  (params (DeltaSeconds :type "Float (single-precision)"))
  (if (`self.Toggle`)
    (switch `/Game/BlueprintEX/EN_MoveType` (`self.MoveType`)
      (:`NewEnumerator0`
        (`self.RtoU`))
      (:`NewEnumerator1`
        (`self.UtoL`))
      (:`NewEnumerator2`
        (`self.LtoD`))
      (:`NewEnumerator3`
        (`self.DtoR`)))))

(event `self.ReceiveBeginPlay`
  (`self.GetDataFromDispatcherOfSwitch`))

(fn `DtoR`
  (set `self.Z` (+ (`self.Z`) -10.0))
  (`SceneComponent.K2_AddRelativeLocation` (`self.Cube`) (0.0 0.0 -10.0) false false)
  (if (< (`self.Z`) 0.0)
    (set `self.MoveType` "NewEnumerator0")))

(fn `GetDataFromDispatcherOfSwitch`
  (add `/Game/BlueprintEX/BlueprintInterface/BP_Switch.NewEventDispatcher_Toggle` (`self.Switch`) (`|CreateDelegate` :!event `SwitchToggle`)))

(fn `LtoD`
  (set `self.X` (+ (`self.X`) -10.0))
  (`SceneComponent.K2_AddRelativeLocation` (`self.Cube`) (-10.0 0.0 0.0) false false)
  (if (< (`self.X`) 0.0)
    (set `self.MoveType` "NewEnumerator3")))

(fn `RtoU`
  (set `self.X` (+ (`self.X`) 10.0))
  (`SceneComponent.K2_AddRelativeLocation` (`self.Cube`) (10.0 0.0 0.0) false false)
  (if (> (`self.X`) 150.0)
    (set `self.MoveType` "NewEnumerator1")))

(fn `SwitchToggle`
  (params (NewParam :type Boolean))
  (set `self.Toggle` NewParam))

(fn `UserConstructionScript`)

(fn `UtoL`
  (set `self.Z` (+ (`self.Z`) 10.0))
  (`SceneComponent.K2_AddRelativeLocation` (`self.Cube`) (0.0 0.0 10.0) false false)
  (if (> (`self.Z`) 150.0)
    (set `self.MoveType` "NewEnumerator2")))