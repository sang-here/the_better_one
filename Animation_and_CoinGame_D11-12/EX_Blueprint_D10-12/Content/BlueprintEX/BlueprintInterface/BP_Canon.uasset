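; BP_Canon is a rotating-barrel cannon that shows an F-key fire prompt on trigger overlap and toggles firing through SwitchTriggerwithPressF.
; Toggling on spins the barrels through a sine spin-up timeline, then a restarting loop timeline.
; Spin-up updates set looping timers that spawn balls and shells from arrow components, scaled by Fastforward, and snap the cannon to overlapping Characters' meshes.
; Toggling off clears those timers and stops only the loop timeline.
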(event `self.CanonTrigger.OnComponentBeginOverlap`
  (params (OverlappedComponent :type "PrimitiveComponent Object Reference") (OtherActor :type "Actor Object Reference") (OtherComp :type "PrimitiveComponent Object Reference") (OtherBodyIndex :type Integer) (bFromSweep :type Boolean) (SweepResult :type "HitResult Structure (by ref)"))
  (`KismetSystemLibrary.PrintString` "Please Press F to fire"))

(event `/Game/BlueprintEX/BPI_Switch.SwitchTriggerWithPressF`
  (bind _output_get (set `self.Toggle` (not (`self.Toggle`))))
  (if _output_get
    (bind (_direction _sine) (`Timeline|Timeline_BarrelsRotation_sine`)
      (:`Update`
        (`SceneComponent.K2_AddRelativeRotation` (`self.Barrels`) (`KismetMathLibrary.MakeRotator` 0.0 0.0 (* (* (`KismetMathLibrary.DegSin` (* _sine (/ (`KismetMathLibrary.GetPI`) 2.0))) -10.0) (* 1.0 (`self.Fastforward`)))) false false)
        (`KismetSystemLibrary.K2_SetTimer` null "CanonBallShellShooter" (/ 0.5 (`self.Fastforward`)) true)
        (`KismetSystemLibrary.K2_SetTimer` null "CanonShooter" (/ 0.5 (`self.Fastforward`)) true)
        (`KismetSystemLibrary.K2_SetTimer` null "HoldCanon" 0.001 true))
      (:`Finished`
        (bind (_direction_2 _sine_2) (`Timeline|Timeline_BarrelsRotation` :!label _label)
          (:`Update`
            (`SceneComponent.K2_AddRelativeRotation` (`self.Barrels`) (`KismetMathLibrary.MakeRotator` 0.0 0.0 (* (* _sine_2 -10.0) (* 1.0 (`self.Fastforward`)))) false false))
          (:`Finished`
            (goto _label :!via `PlayFromStart`)))))
    (else
      (`|ExecutionSequence`
        (:`then_0`
          (`KismetSystemLibrary.K2_ClearTimer` null "CanonBallShellShooter")
          (`KismetSystemLibrary.K2_ClearTimer` null "CanonShooter")
          (`KismetSystemLibrary.K2_ClearTimer` null "HoldCanon"))
        (:`then_1`
          (goto _label :!via `Stop`))))))

(fn `CanonBallShellShooter`
  (bind (_returnvalue_location _returnvalue_rotation) (`KismetMathLibrary.BreakTransform` (`SceneComponent.K2_GetComponentToWorld` (`self.ShellEjectionPortArrow`))))
  (`|SpawnActorFromClass` "/Game/BlueprintEX/BlueprintInterface/BP_CanonBallShell.BP_CanonBallShell_C" (`KismetMathLibrary.MakeTransform` _returnvalue_location _returnvalue_rotation) "Undefined" "MultiplyWithRoot" null null))

(fn `CanonShooter`
  (bind (_returnvalue_location _returnvalue_rotation) (`KismetMathLibrary.BreakTransform` (`SceneComponent.K2_GetComponentToWorld` (`self.CanonBallEjectionPointArrow`))))
  (`|SpawnActorFromClass` "/Game/BlueprintEX/BlueprintInterface/BP_CanonBall.BP_CanonBall_C" (`KismetMathLibrary.MakeTransform` _returnvalue_location _returnvalue_rotation) "Undefined" "MultiplyWithRoot" null null))

(fn `HoldCanon`
  (for _array_element (`PrimitiveComponent.GetOverlappingActors` (`self.CanonTrigger`) null)
    (bind _ascharacter (cast `Character` _array_element))
    (bind _returnvalue (`SceneComponent.K2_GetComponentToWorld` (`Character.Mesh` _ascharacter)))
    (`SceneComponent.K2_SetWorldTransform` (`self.DefaultSceneRoot`) (`KismetMathLibrary.MakeTransform` (`KismetMathLibrary.MakeVector` (.x (.location _returnvalue)) (+ (.y (.location _returnvalue)) 40.0) (+ (.z (.location _returnvalue)) 58.0)) (`KismetMathLibrary.MakeRotator` 0.0 0.0 (+ (.yaw (.rotation _returnvalue)) -90.0))) false false)))

(fn `UserConstructionScript`)