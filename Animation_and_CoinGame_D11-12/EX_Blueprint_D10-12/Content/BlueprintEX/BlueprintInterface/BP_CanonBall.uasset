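; BP_CanonBall is a physics cannonball projectile that knocks back the third-person character on impact.
; On BeginPlay it launches its Sphere with a forward impulse and starts a one-shot timer that calls RemoveBall to destroy the actor after a few seconds.
; When the Sphere hits a BP_ThirdPersonCharacter, it prints that actor's name and applies the reversed, scaled hit normal impulse to the character's movement component.
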(event `self.ReceiveBeginPlay`
  (bind _sphere (`self.Sphere`))
  (`PrimitiveComponent.AddImpulse` _sphere (* (`SceneComponent.GetForwardVector` _sphere) 15000.0) "None" false)
  ;[0.15 0.15 0.15 0.5 12] 여기서는 looping off to use it as a delay
  (`KismetSystemLibrary.K2_SetTimer` null "RemoveBall" 5.0))

(event `self.Sphere.OnComponentHit`
  (params (HitComponent :type "PrimitiveComponent Object Reference") (OtherActor :type "Actor Object Reference") (OtherComp :type "PrimitiveComponent Object Reference") (NormalImpulse :type "Vector Structure") (Hit :type "HitResult Structure (by ref)"))
  (bind _asbp_third_person_character (cast `/Game/ThirdPerson/Blueprints/BP_ThirdPersonCharacter` OtherActor))
  (`KismetSystemLibrary.PrintString` (`KismetSystemLibrary.GetDisplayName` OtherActor))
  (`CharacterMovementComponent.AddImpulse` (`Character.CharacterMovement` _asbp_third_person_character) (* NormalImpulse -2.0) false))

(fn `RemoveBall`
  (`self.K2_DestroyActor`))

(fn `UserConstructionScript`)