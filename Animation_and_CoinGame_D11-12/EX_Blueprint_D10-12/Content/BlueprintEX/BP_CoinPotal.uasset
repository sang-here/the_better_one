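; Coin-gated portal whose Sphere opens Lvl_ThirdPerson when overlapped.
; BeginPlay hides the Sphere, disables its collision and binds to every BP_Coin's get-coin dispatcher.
; CheckCoin shows the Sphere when GetRemainCoin finds no coins outside those being destroyed, but enables collision regardless of count.
; Older counting functions and disconnected event nodes remain alongside this logic.
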(event `self.Sphere.OnComponentBeginOverlap`
  (params (OverlappedComponent :type "PrimitiveComponent Object Reference") (OtherActor :type "Actor Object Reference") (OtherComp :type "PrimitiveComponent Object Reference") (OtherBodyIndex :type Integer) (bFromSweep :type Boolean) (SweepResult :type "HitResult Structure (by ref)"))
  (`KismetSystemLibrary.PrintString` "Hello")
  (`GameplayStatics.OpenLevel` "Lvl_ThirdPerson"))

(event `self.ReceiveBeginPlay`
  ; V1
  (`SceneComponent.SetVisibility` (`self.Sphere`) false false)
  ; V4
  (`PrimitiveComponent.SetCollisionEnabled` (`self.Sphere`) "NoCollision")
  ; V3
  (bind _outactors (`GameplayStatics.GetAllActorsOfClass` "/Game/BlueprintEX/BP_Coin.BP_Coin_C"))
  (for _array_element _outactors
    (add `/Game/BlueprintEX/BP_Coin.NewEventDispatcherGetCoin` _array_element (`|CreateDelegate` :!event `CheckCOin`))))

(fn `CheckCoin`
  (`SceneComponent.SetVisibility` (`self.Sphere`) (== (`self.GetRemainCoin`) 0) false)
  (`PrimitiveComponent.SetCollisionEnabled` (`self.Sphere`) "QueryAndPhysics"))

(fn `CoinOpenPortal`
  (bind _outactors (`GameplayStatics.GetAllActorsOfClass` "/Game/BlueprintEX/BP_Coin.BP_Coin_C"))
  (for (_ _array_index) _outactors
    (bind _output_get (set `self.HowManyCoin` (+ _array_index 1)))
    (set `self.TotalCoinRemain` _output_get))
  (if (== (`self.HowManyCoin`) 0)
    (`SceneComponent.SetVisibility` (`self.Sphere`) true false)
    (else
      (set `self.HowManyCoin` 0))))

(fn `EventCoinOpenPortal`
  (params (NewParam :type Boolean))
  (if NewParam
    (bind _outactors (`GameplayStatics.GetAllActorsOfClass` "/Game/BlueprintEX/BP_Coin.BP_Coin_C"))
    (for (_ _array_index) _outactors
      (set `self.HowManyCoin` (+ _array_index 1)))
    (if (== (`self.HowManyCoin`) 0)
      (`SceneComponent.SetVisibility` (`self.Sphere`) true false)
      (else
        (set `self.HowManyCoin` 0)))))

(fn `GetRemainCoin`
  (returns (OutActors :type Integer))
  (locals (Coin :type Integer))
  (bind _outactors (`GameplayStatics.GetAllActorsOfClass` "/Game/BlueprintEX/BP_Coin.BP_Coin_C"))
  (for _array_element _outactors
    (if (not (`self.IsActorBeingDestroyed` _array_element))
      (set `local.Coin` (+ (`local.Coin`) 1))))
  (return (`local.Coin`)))

(fn `GetTotalCoinAtBegining`
  (bind _outactors (`GameplayStatics.GetAllActorsOfClass` "/Game/BlueprintEX/BP_Coin.BP_Coin_C"))
  (for (_ _array_index) _outactors
    (bind _output_get (set `self.HowManyCoin` (+ _array_index 1)))
    (set `self.TotalCoinRemain` _output_get)))

(fn `UserConstructionScript`)