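; BP_PortalV3 is a password portal whose Sphere is hidden at start and shown when the counts of the CountingBox actors match the password.
; BeginPlay binds an event to each box's dispatcher through FromCountingToggle.
; OnPotalV3 sets visibility from IndexPassword, which compares each count to a digit of the integer Password1, extracted with modulo and powers of ten.
; An older V2 event instead compares every count to the Password array's first element.
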(event `OnPotalV3`
  ; V3
  (bind _newparam (`self.IndexPassword`))
  (`KismetSystemLibrary.PrintString` "@@@@@@")
  (`SceneComponent.SetVisibility` (`self.Sphere`) _newparam false))

(event `CustomEvent_1`
  ; V2
  (bind _newparam (`self.369 by array`))
  (`KismetSystemLibrary.PrintString` "@@@@@@")
  (`SceneComponent.SetVisibility` (`self.Sphere`) _newparam false))

(event `self.ReceiveBeginPlay`
  ; V3
  (`SceneComponent.SetVisibility` (`self.Sphere`) false false)
  (`self.FromCountingToggle`))

(event `CustomEvent`
  ; V2
  (`SceneComponent.SetVisibility` (`self.Sphere`) false false)
  (`self.FromCountingToggle`))

(fn `369 by array`
  (returns (NewParam :type Boolean))
  (for _array_element (`self.CountingBox`)
    (if (not (== (`/Game/BlueprintEX/CountingPotalV3/BP_CountingV3.count` _array_element) (`|GetArrayItem` (`self.password`))))
      (return false)))
  (return true))

(fn `BP_PortalPassword_AutoGenFunc`
  (params (PortalOnOff :type Boolean))
  (set `self.PortalOnOff` PortalOnOff))

(fn `FromCountingToggle`
  (for _array_element (`self.CountingBox`)
    (add `/Game/BlueprintEX/CountingPotalV3/BP_CountingV3.NewEventDispatcherFromCounting10Password` _array_element (`|CreateDelegate` :!event `BP_PortalPassword_AutoGenFunc`))))

(fn `GetIndexPass`
  (params (Index :type Integer))
  (returns (SinglePassword :type Integer))
  (bind _returnvalue (- (`KismetArrayLibrary.Array_Length` (`self.CountingBox`)) Index))
  (return (/ (mod (`self.Password1`) (`self.NPowerOf10` _returnvalue)) (`self.NPowerOf10` (- _returnvalue 1)))))

(fn `IndexPassword`
  (returns (NewParam :type Boolean))
  (for (_array_element _array_index) (`self.CountingBox`)
    (if (not (== (`/Game/BlueprintEX/CountingPotalV3/BP_CountingV3.count` _array_element) (`self.GetIndexPass` _array_index)))
      (return false)))
  (return true))

(fn `NPowerOf10`
  (params (multiplyCnt :type Integer))
  (returns (Cnt10 :type Integer))
  (locals (LocalCnt10 :type Integer :default 1))
  (for _ (range 1 (+ multiplyCnt 1))
    (set `local.LocalCnt10` (* (`local.LocalCnt10`) 10)))
  (return (`local.LocalCnt10`)))

(fn `UserConstructionScript`)