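; BP_Timer is an event dispatcher example actor that shows a running MM:SS timer on a TextRender, advancing at ten times real speed.
; On BeginPlay it binds to the toggle dispatcher of a referenced Switch, with an auto-generated handler that sets the Toggle flag.
; While Toggle is true, Tick accumulates scaled delta time and rewrites the text using a zero-padding helper function.
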(event `self.ReceiveTick`
  (params (DeltaSeconds :type "Float (single-precision)"))
  (if (`self.Toggle`)
    (bind _output_get (set `self.TotalDeltaSeconds` (+ (`self.TotalDeltaSeconds`) (* DeltaSeconds 10.0))))
    (`TextRenderComponent.K2_SetText` (`self.TextRender`) (`KismetTextLibrary.Conv_StringToText` (`KismetStringLibrary.Concat_StrStr` (`self.FloatToStrZeroN` (/ _output_get 60.0)) ":" (`self.FloatToStrZeroN` (mod _output_get 60.0)))))))

(event `self.ReceiveBeginPlay`
  (`self.SwitchToggle`))

(fn `BP_Timer_AutoGenFunc`
  (params (NewParam :type Boolean))
  (set `self.Toggle` NewParam))

(fn `FloatToStrZeroN`
  (params (Number :type "Float (double-precision)"))
  (returns (Str00 :type String))
  (bind _returnvalue (`KismetStringLibrary.Conv_IntToString` (`KismetMathLibrary.FFloor` Number)))
  (if (< Number 10.0)
    (return (`KismetStringLibrary.Concat_StrStr` "0" _returnvalue))
    (else
      (return _returnvalue))))

(fn `SwitchToggle`
  (add `/Game/BlueprintEX/BlueprintInterface/BP_Switch.NewEventDispatcher_Toggle` (`self.Switch`) (`|CreateDelegate` :!event `BP_Timer_AutoGenFunc`)))

(fn `UserConstructionScript`)