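; Tens-style password counter Blueprint (D10) for a counting portal puzzle, advanced by an F-press switch trigger.
; Each trigger increments Count, wraps it from 9 to 0, updates the text render, then calls OnPotal on the linked BPPotalD10.
; An older V1 check for a 3-6-9 combination and a dispatcher call remain in the graph but are disconnected.
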(event `self.SwitchTriggerWithPressF`
  ; V2
  (`self.Till9Plus1`)
  (`/Game/BlueprintEX/CountingPotalV2/BP_Portal_PasswordD10.OnPotal` (`self.BP_Potal_d10`)))

(fn `IfAll9OrNotTo369`
  (returns (AllBox9 :type Boolean))
  (for (_ _array_index) (`self.CountingD10`)
    (if (== _array_index 0)
      (if (== (`self.count`) 3)
        (bind _output_get (set `self.If 3` true))
        (else
          (set `self.If 3` false)))
      (if (and _output_get (stale _output_get_2) (stale _output_get_3)) :!label _label
        (`KismetSystemLibrary.PrintString` "Hello")
        (return true))
      (elif (== _array_index 1)
        (if (== (`self.count`) 6)
          (bind _output_get_2 (set `self.If 6` true))
          (goto _label)
          (else
            (set `self.If 6` false)
            (goto _label)))
        (elif (== _array_index 2)
          (if (== (`self.count`) 9)
            (bind _output_get_3 (set `self.If 9` true))
            (goto _label)
            (else
              (set `self.If 9` false)
              (goto _label))))))))

(fn `Till9Plus1`
  (set `self.count` (+ (`self.count`) 1))
  (if (== (`self.count`) 10)
    (set `self.count` 0))
  (`TextRenderComponent.K2_SetText` (`self.TextRender`) (`KismetTextLibrary.Conv_IntToText` (`self.count`))))

(fn `UserConstructionScript`)